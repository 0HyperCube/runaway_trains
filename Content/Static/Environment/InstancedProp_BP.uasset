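; Environment prop actor that randomly scatters Count instances of a static mesh across a fixed world-space rectangle, keeping them off the track.
; The construction script clears and rebuilds the instances, giving each random yaw and uniform scale within ScaleRange.
; Rejection sampling rerolls any point within a fixed distance of a TrackSegement spline, using a cached spline list.
; The closest spline point is queried in local space but compared to the world-space candidate.
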(event EventBeginPlay)

(event Collision|EventActorBeginOverlap
  (params (OtherActor :type Actor%20Object%20Reference)))

(event EventTick
  (params (DeltaSeconds :type Float%20%28single-precision%29)))

(fn ConstructionScript
  (bind _returnvalue (Math|Transform|MakeTransform "0, 0, 0"))
  (bind _scalerange (Variables|Generation|GetScaleRange))
  (Components|InstancedStaticMesh|ClearInstances (Variables|Default|GetInstancedStaticMesh))
  (for _index (range 0 (Variables|Generation|GetCount))
    (Variables|Default|SetNewVar_0 _returnvalue)
    (while (or (Class|KismetMathLibrary|NearlyEqualTransformTransform (Variables|Default|GetNewVar_0) _returnvalue 0.0001 0.0001 0.0001) (stale _return))
      (bind _output_get (Variables|Default|SetNewVar_0 (Math|Transform|MakeTransform (Math|Vector|MakeVector (Math|Random|RandomFloatinRange 1.2e+04 4e+04) (Math|Random|RandomFloatinRange 8e+03 2.8e+04) 0.0) (Math|Rotator|MakeRotator 0.0 0.0 (Math|Random|RandomFloatinRange 0.0 3.6e+02)) (Math|Conversions|ToVector(Float) (Math|Random|RandomFloatinRange (.x _scalerange) (.y _scalerange))))))
      (bind _return (CallFunction|PointIsonTrack _output_get)))
    (Class|InstancedStaticMeshComponent|AddInstanceWorldSpace (Variables|Default|GetInstancedStaticMesh) (Variables|Default|GetNewVar_0))))

(fn PointIsonTrack
  (params (point :type Transform))
  (Utilities|FlowControl|Sequence
    (:then_0
      (if (not (> (Utilities|Array|Length (Variables|Default|GetNewVar_1)) 0))
        (bind _outactors (Actor|GetAllActorsOfClass "/Script/TrainTragedy.TrackSegement"))
        (for _array_element _outactors
          (Utilities|Array|Add (Variables|Default|GetNewVar_1) (Variables|/Script/TrainTragedy.TrackSegement|GetSplineComponent _array_element)))))
    (:then_1
      (for _array_element_2 (Variables|Default|GetNewVar_1)
        (bind _location (CallFunction|GetDistanceAlongSplineClosesttoWorldPosition (.location point) _array_element_2))
        (if (< (Math|Vector|Distance(Vector) _location (.location point)) 1.5e+03)
          (return true)))
      (return false))))

(fn GetDistanceAlongSplineClosesttoWorldPosition
  (params (World%20Position :type Vector) (Spline :type Spline%20Component%20Object%20Reference))
  (return (.location (Class|SplineComponent|FindTransformClosesttoWorldLocation Spline World%20Position "Local" false))))