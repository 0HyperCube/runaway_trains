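; Player pawn that lets the player click track-style SegementConnector actors and can glide its view to a target transform.
; BeginPlay enables input in UI-only mode, and SelectPoints line-traces from the cursor to call ChangeDirection on the connector hit, printing debug text.
; MoveToLocation records the start transform, then Tick keeps calling it to blend location and control rotation toward TargetLocation over three seconds with ease-in-out, snapping at the end.
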(event EventBeginPlay
  (bind _returnvalue (Game|GetPlayerController 0))
  (Input|EnableInput _returnvalue)
  (Input|SetInputModeUIOnly _returnvalue 0 "DoNotLock"))

(event Collision|EventActorBeginOverlap
  (params (OtherActor :type Actor%20Object%20Reference)))

(event EventTick
  (params (DeltaSeconds :type Float%20%28single-precision%29))
  (if (Variables|Default|GetbIsGliding)
    (CallFunction|MovetoLocation)))

(event Input|ActionEvents|InputActionSelectPoints
  (params (Key :type Key%20Structure :default "None"))
  (bind _returnvalue (Game|GetPlayerController 0))
  (bind (_worldlocation _worlddirection) (Game|Player|ConvertMouseLocationToWorldSpace _returnvalue))
  (:Pressed
    (Development|PrintString "points")
    (bind (_outhit _returnvalue_2) (Collision|LineTraceByChannel _worldlocation (+ _worldlocation (* _worlddirection 5000000)) "TraceTypeQuery3" false 0 "None"))
    (if _returnvalue_2
      (bind _assegement_connector (Utilities|Casting|CastToSegementConnector (.hitactor _outhit))
        (:then
          (Class|SegementConnector|ChangeDirection _assegement_connector)
          (Development|PrintString "changed dir"))
        (:CastFailed
          (Development|PrintString (Utilities|GetDisplayName (.hitactor _outhit)) :!label _label)))
      (else
        (goto _label)))))

(fn ConstructionScript)

(fn MovetoLocation
  (bind _targetlocation (Variables|Default|GetTargetLocation))
  (bind _targetlocation_2 (Variables|Default|GetTargetLocation))
  (Utilities|FlowControl|Sequence
    (:then_0
      (if (not (Variables|Default|GetbIsGliding))
        (Variables|Default|SetTimeStarted (Utilities|Time|GetRealTimeSeconds))
        (Variables|Default|SetbIsGliding true)
        (Variables|Default|SetStartTransform (Math|Transform|MakeTransform (Transformation|GetActorLocation) (Pawn|GetDesiredRotation (Game|GetPlayerController 0)) "1,1,1"))))
    (:then_1
      (if (< (/ (- (Utilities|Time|GetRealTimeSeconds) (Variables|Default|GetTimeStarted)) 3.0) 1.0)
        (Transformation|SetActorLocation (Math|Vector|Lerp(Vector) (.location (Variables|Default|GetStartTransform)) (.location _targetlocation_2) (Utilities|EaseinOut (/ (- (Utilities|Time|GetRealTimeSeconds) (Variables|Default|GetTimeStarted)) 3.0) 3.0)) false false)
        (Pawn|SetControlRotation (Game|GetPlayerController 0) (Math|Rotator|Lerp(Rotator) (.rotation (Variables|Default|GetStartTransform)) (.rotation _targetlocation_2) (Utilities|EaseinOut (/ (- (Utilities|Time|GetRealTimeSeconds) (Variables|Default|GetTimeStarted)) 3.0) 3.0) true))
        (else
          (Transformation|SetActorLocation (.location _targetlocation) false false)
          (Pawn|SetControlRotation (Game|GetPlayerController 0) (.rotation _targetlocation))
          (Variables|Default|SetbIsGliding false))))))