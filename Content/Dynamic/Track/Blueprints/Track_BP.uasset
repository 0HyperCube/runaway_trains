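; Railway track actor that builds rails and sleepers along a spline when its RedrawGraphics event runs.
; CreateSleepers places evenly spaced, spline-aligned mesh instances, with a tiny random Z offset on the whole instanced component.
; CreateRails chains spline mesh segments along the curve, stretching the nominal segment length to fit a whole count.
; Both functions reuse existing pieces, add missing ones and run a cleanup loop intended to trim the surplus.
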(event EventBeginPlay)

(event Collision|EventActorBeginOverlap
  (params (OtherActor :type Actor%20Object%20Reference)))

(event EventTick
  (params (DeltaSeconds :type Float%20%28single-precision%29)))

(event EventRedrawGraphics
  (CallFunction|CreateSleepers)
  (CallFunction|CreateRails))

(fn ConstructionScript
  (|CallParentFunction))

(fn CreateRails
  (bind _rail_spline_meshes (Variables|Default|GetRail%20Spline%20Meshes))
  (bind _rail_segement_length (Variables|Default|GetRail%20Segement%20Length))
  (bind _splinecomponent (Variables|Default|GetSplineComponent))
  (bind _splinecomponent_2 (Variables|Default|GetSplineComponent))
  (bind _splinecomponent_3 (Variables|Default|GetSplineComponent))
  (bind _returnvalue (Spline|GetSplineLength _splinecomponent_3))
  (bind _returnvalue_2 (/ _returnvalue _rail_segement_length))
  (bind _returnvalue_3 (Math|Float|Floor _returnvalue_2))
  (bind _returnvalue_4 (- _returnvalue_3 1))
  (for _index (range 0 _returnvalue_4)
    (Utilities|FlowControl|Sequence
      (:then_0
        ;[1 1 1] Create new spline meshes
        (if (not (Utilities|Array|IsValidIndex (Variables|Default|GetRail%20Spline%20Meshes) _index))
          (bind _returnvalue_5 (AddComponent|AddSplineMeshComponent false (Math|Transform|MakeTransform "0, 0, 0")))
          (Components|StaticMesh|SetStaticMesh _returnvalue_5 "/Game/Dynamic/Track/Model/RailSegement.RailSegement")
          (Utilities|Array|SetArrayElem (Variables|Default|GetRail%20Spline%20Meshes) _index _returnvalue_5 true)))
      (:then_1
        ;[1 1 1] Position spline meshes
        (SplineMesh|SetStartandEnd (Utilities|Array|Get(acopy) (Variables|Default|GetRail%20Spline%20Meshes) _index) (Spline|GetLocationatDistanceAlongSpline _splinecomponent (LocalVariables|Getend%20point) "World") (Spline|GetDirectionatDistanceAlongSpline _splinecomponent (LocalVariables|Getend%20point) "Local") (Spline|GetLocationatDistanceAlongSpline _splinecomponent_2 (+ (LocalVariables|Getend%20point) (/ _returnvalue (Math|Conversions|ToFloat(Integer) _returnvalue_3))) "World") (Spline|GetDirectionatDistanceAlongSpline _splinecomponent_2 (+ (LocalVariables|Getend%20point) (/ _returnvalue (Math|Conversions|ToFloat(Integer) _returnvalue_3))) "Local") true :!class /Script/Engine.SplineMeshComponent)
        (LocalVariables|Setend%20point (+ (LocalVariables|Getend%20point) (/ _returnvalue (Math|Conversions|ToFloat(Integer) _returnvalue_3)))))))
  (for _index_2 (range _returnvalue_4 (Utilities|Array|Length (Variables|Default|GetRail%20Spline%20Meshes)))
    (Components|DestroyComponent (Utilities|Array|Get(acopy) _rail_spline_meshes _index_2))
    (Utilities|Array|RemoveIndex _rail_spline_meshes _index_2)))

(fn CreateSleepers
  (bind _sleeper_distance (Variables|Default|GetSleeper%20Distance))
  (bind _sleepers (Variables|Default|GetSleepers))
  (bind _splinecomponent (Variables|Default|GetSplineComponent))
  (bind _splinecomponent_2 (Variables|Default|GetSplineComponent))
  (bind _returnvalue (Spline|GetSplineLength _splinecomponent_2))
  (bind _returnvalue_2 (/ _returnvalue _sleeper_distance))
  (bind _returnvalue_3 (Math|Float|Floor _returnvalue_2))
  (bind _returnvalue_4 (Math|Conversions|ToFloat(Integer) _returnvalue_3))
  (bind _returnvalue_5 (- _returnvalue_3 1))
  (bind _returnvalue_6 (/ _returnvalue _returnvalue_4))
  (Utilities|FlowControl|Sequence
    (:then_0
      ;[1 1 1] Reset transform
      (Transformation|SetRelativeLocationAndRotation _sleepers (Math|Vector|MakeVector 0.0 0.0 (Math|Random|RandomFloatinRange -0.0001 0.1001)) (Transformation|GetActorRotation) false false)
      (for _index (range 0 _returnvalue_5)
        (if (>= _index (Components|InstancedStaticMesh|GetInstanceCount _sleepers))
          (Class|InstancedStaticMeshComponent|AddInstanceWorldSpace _sleepers (Math|Transform|MakeTransform (Spline|GetLocationatDistanceAlongSpline _splinecomponent (+ (* _index _returnvalue_6) (/ _returnvalue_6 2.0)) "World") (Math|Conversions|RotationFromXVector (Spline|GetDirectionatDistanceAlongSpline _splinecomponent (+ (* _index _returnvalue_6) (/ _returnvalue_6 2.0)) "Local"))))
          (else
            (Components|InstancedStaticMesh|UpdateInstanceTransform _sleepers _index (Math|Transform|MakeTransform (Spline|GetLocationatDistanceAlongSpline _splinecomponent (+ (* _index _returnvalue_6) (/ _returnvalue_6 2.0)) "World") (Math|Conversions|RotationFromXVector (Spline|GetDirectionatDistanceAlongSpline _splinecomponent (+ (* _index _returnvalue_6) (/ _returnvalue_6 2.0)) "Local"))) true false true)))))
    (:then_1
      (for _index_2 (range _returnvalue_5 (- (Components|InstancedStaticMesh|GetInstanceCount (Variables|Default|GetSleepers)) 1))
        (Class|InstancedStaticMeshComponent|RemoveInstance (Variables|Default|GetSleepers) _index_2)))))