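; Track actor that builds a segmented track mesh along a spline in the construction script.
; It divides the spline length by a segment length and adds a spline mesh component for each whole segment, with start and end positions sampled by distance in local space.
; Tangents are left unconnected, and a debug print reports the piece count.
; The event graph holds no runtime logic.
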(event EventBeginPlay)

(event Collision|EventActorBeginOverlap
  (params (OtherActor :type Actor%20Object%20Reference)))

(event EventTick
  (params (DeltaSeconds :type Float%20%28single-precision%29)))

(fn ConstructionScript
  (bind _spline (Variables|Default|GetSpline))
  (bind _spline_2 (Variables|Default|GetSpline))
  (bind _segement_length (Variables|Default|GetSegement%20Length))
  (bind _returnvalue (Spline|GetSplineLength _spline_2))
  (bind _returnvalue_2 (/ _returnvalue _segement_length))
  (bind _returnvalue_3 (Math|Float|Floor _returnvalue_2))
  (bind _returnvalue_4 (- _returnvalue_3 1))
  (Development|PrintString (Utilities|String|Append "Construct peices: " (Utilities|String|ToString(Integer) _returnvalue_4)))
  (for _index (range 0 _returnvalue_4)
    (Utilities|FlowControl|Sequence
      (:then_0
        (bind _returnvalue_5 (AddComponent|AddSplineMeshComponent false))
        (SplineMesh|SetStartandEnd _returnvalue_5 (Spline|GetLocationatDistanceAlongSpline _spline (* _index (Variables|Default|GetSegement%20Length)) "Local") "0, 0, 0" (Spline|GetLocationatDistanceAlongSpline _spline (+ (* _index (Variables|Default|GetSegement%20Length)) (Variables|Default|GetSegement%20Length)) "Local") "0, 0, 0" true :!class /Script/Engine.SplineMeshComponent)))))