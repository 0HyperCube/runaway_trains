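; BP_TrainCarriage is a train carriage actor that passes its physical collisions on to an OnCompHit handler defined outside this graph.
; The Hit event stores the hit info and raises a flag, which Tick clears before calling OnCompHit, so only the latest hit is handled on the next tick.
; The construction script sets the Cube component to half world scale.
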(event EventBeginPlay)

(event Collision|EventActorBeginOverlap
  (params (OtherActor :type Actor%20Object%20Reference)))

(event EventTick
  (params (DeltaSeconds :type Float%20%28single-precision%29))
  (if (Variables|Default|GetbHasColided)
    (Variables|Default|SetbHasColided false)
    (Class|TrainCarriage|OnCompHit (Variables|Default|GetCollisionInfo))))

(event Collision|EventHit
  (params (MyComp :type Primitive%20Component%20Object%20Reference) (Other :type Actor%20Object%20Reference) (OtherComp :type Primitive%20Component%20Object%20Reference) (bSelfMoved :type Boolean) (HitLocation :type Vector :default "0, 0, 0") (HitNormal :type Vector :default "0, 0, 0") (NormalImpulse :type Vector :default "0, 0, 0") (Hit :type Hit%20Result%20Structure%20%28by%20ref%29))
  (Variables|Default|SetbHasColided true)
  (Variables|Default|SetCollisionInfo Hit))

(fn ConstructionScript
  (Transformation|SetWorldScale3D (Variables|Default|GetCube) "0.500000,0.500000,0.500000"))